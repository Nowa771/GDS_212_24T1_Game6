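; BP_Gate is a double gate that swings open when the level's Button fires its Open dispatcher.
; On BeginPlay it finds the Button with GetActorOfClass and binds its own Open event to that dispatcher.
; Open plays the DoorAnim timeline, whose alpha lerps the yaw of DoorL and DoorR in opposite directions.
; The OpenDoor event is empty, and the delayed call to it never runs.
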(event `self.ReceiveBeginPlay`
  (bind _returnvalue (`GameplayStatics.GetActorOfClass` "/Game/BluePrints/Button.Button_C"))
  (bind _output_get (set `self.Button ref` _returnvalue))
  (add `/Game/BluePrints/Button.Open` _output_get (delegate `Open`)))

(event `Open`
  (bind (_direction _door_rotation) (`Timeline|Door Anim`)
    (:`Update`
      (`SceneComponent.K2_SetRelativeRotation` (`self.Door L`) (`KismetMathLibrary.MakeRotator` 0.0 0.0 (`KismetMathLibrary.Lerp` 0.0 -120.0 _door_rotation)) false false)
      (`SceneComponent.K2_SetRelativeRotation` (`self.Door R`) (`KismetMathLibrary.MakeRotator` 0.0 0.0 (`KismetMathLibrary.Lerp` 0.0 120.0 _door_rotation)) false false))))

(event `Open Door`)

(fn `UserConstructionScript`)